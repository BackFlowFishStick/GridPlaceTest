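; Pawn that lets the player position and place a unit on a BP_GridActor with the mouse.
; While a unit is held, Tick line-traces from the cursor, has the unit check grid status and snaps it to the closest grid location.
; Left-click release tries to place it on the selected tile and clears the held unit on success.
; Right-click release resets the unit's location and clears it.
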(event `self.ReceiveTick`
  (params (DeltaSeconds :type "Float (single-precision)"))
  (bind _placeunit (`self.placeUnit`))
  (bind (_worldlocation _worlddirection) (`PlayerController.DeprojectMousePositionToWorld` (`GameplayStatics.GetPlayerController` 0)))
  (`/Engine/EditorBlueprintResources/StandardMacros.IsValid` (`self.placeUnit`)
    (:`Is Valid`
      (bind (_outhit _returnvalue) (`KismetSystemLibrary.LineTraceSingle` _worldlocation (+ _worldlocation (* (`self.traceLength`) _worlddirection)) "TraceTypeQuery3"))
      (if _returnvalue
        (bind (_bblockinghit _binitialoverlap _time _distance _location _impactpoint _normal _impactnormal _physmat _hitactor) (`GameplayStatics.BreakHitResult` _outhit))
        (bind _asbp_grid_actor (cast `/Game/Blueprints/BP_GridActor` _hitactor))
        (set `self.GridMap` _asbp_grid_actor)
        (`/Game/Blueprints/BP_PlaceUnit.OnCheckingGridStatus` _placeunit _asbp_grid_actor)
        (bind _output (`/Game/Blueprints/BP_GridActor.GetClosetLocationOnGrid` _asbp_grid_actor _location))
        (`self.K2_SetActorLocation` _placeunit _output false true)
        (set `self.SelectedTile` _output)))))

(event `InputAction|MouseLeftClick`
  (params (Key :type "Key Structure"))
  (bind _placeunit (`self.placeUnit`))
  (:`Released`
    (`/Engine/EditorBlueprintResources/StandardMacros.IsValid` _placeunit
      (:`Is Valid`
        (bind _isreadytoplace (`/Game/Blueprints/BP_PlaceUnit.PlaceObject` _placeunit (`self.SelectedTile`) (`self.GridMap`)))
        (if _isreadytoplace
          (`self.SetPlaceUnit` null)
          (else
            (`KismetSystemLibrary.PrintString` "Hello")))))))

(event `InputAction|MouseRightClick`
  (params (Key :type "Key Structure"))
  (bind _placeunit (`self.placeUnit`))
  (:`Released`
    (`/Engine/EditorBlueprintResources/StandardMacros.IsValid` _placeunit
      (:`Is Valid`
        (`/Game/Blueprints/BP_PlaceUnit.ResetLocation` _placeunit)
        (bind _returnvalue (`self.SetPlaceUnit` null))
        (if _returnvalue
          _)))))

(fn `SetPlaceUnit`
  (params (placeUnit :type "/Game/Blueprints/BP_PlaceUnit Object Reference"))
  (returns (ReturnValue :type Boolean))
  (bind _output_get (set `self.placeUnit` placeUnit))
  (return (`KismetSystemLibrary.IsValid` _output_get)))

(fn `UserConstructionScript`)