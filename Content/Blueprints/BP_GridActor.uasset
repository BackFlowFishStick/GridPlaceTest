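; Grid actor that lays out a GridX by GridY field of tiles and tracks which cells are occupied.
; The construction script adds an instance to Grid for each cell, spaced by TileSize, and caches its position as the component's world location plus an unrotated offset.
; Functions add, remove and check occupied locations by exact vector match, accepting only cached cells.
; A nearest-cell lookup linearly scans the cached locations by distance.
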(fn `AddOccupiedGrid`
  (params (gridLocation :type "Vector Structure"))
  (if (!= (`KismetArrayLibrary.Array_Find` (`self.GridLocations`) gridLocation) -1)
    (`KismetArrayLibrary.Array_AddUnique` (`self.OccupiedLocations`) gridLocation)))

(fn `CheckOccupiedGrid`
  (params (targetGrid :type "Vector Structure"))
  (returns (isOccupied :type Boolean))
  (return (!= (`KismetArrayLibrary.Array_Find` (`self.OccupiedLocations`) targetGrid) -1)))

(fn `GetClosetLocationOnGrid`
  (params (location :type "Vector Structure"))
  (returns (Output :type "Vector Structure"))
  (locals (closestDistance :type "Float (double-precision)" :default 1000.0) (selectedLocationIdx :type Integer))
  (bind _gridlocations (`self.GridLocations`))
  (for (_array_element _array_index) _gridlocations
    (bind _returnvalue (`KismetMathLibrary.Vector_Distance` location _array_element))
    (if (< _returnvalue (`local.closestDistance`))
      (set `local.closestDistance` _returnvalue)
      (set `local.selectedLocationIdx` _array_index)))
  (return (`|GetArrayItem` _gridlocations (`local.selectedLocationIdx`))))

(fn `RemoveOccupiedGrid`
  (params (occupiedGrid :type "Vector Structure"))
  (bind _occupiedlocations (`self.OccupiedLocations`))
  (bind _returnvalue (`KismetArrayLibrary.Array_Find` _occupiedlocations occupiedGrid))
  (if (!= _returnvalue -1)
    (`KismetArrayLibrary.Array_Remove` _occupiedlocations _returnvalue)))

(fn `UserConstructionScript`
  (bind _grid (`self.Grid`))
  (`KismetArrayLibrary.Array_Clear` (`self.GridLocations`))
  (for _index (range (`self.Grid_X`))
    (for _index_2 (range (`self.Grid_Y`))
      (bind _returnvalue (`KismetMathLibrary.MakeTransform` (`KismetMathLibrary.MakeVector` (`KismetMathLibrary.Conv_IntToDouble` (* _index (`self.TileSize`))) (`KismetMathLibrary.Conv_IntToDouble` (* _index_2 (`self.TileSize`))))))
      (`InstancedStaticMeshComponent.AddInstance` _grid _returnvalue false)
      (`KismetArrayLibrary.Array_Add` (`self.GridLocations`) (+ (`SceneComponent.K2_GetComponentLocation` _grid) (`KismetMathLibrary.MakeVector` (.x (.location _returnvalue)) (.y (.location _returnvalue))))))))