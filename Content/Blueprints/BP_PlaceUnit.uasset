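; BP_PlaceUnit is a placeable unit with a GridX by GridY footprint of tile meshes that show whether it fits on a grid.
; The construction script builds the glowing tiles under GridMeshParent, initially red.
; OnCheckingGridStatus queries the passed grid at each tile, colors it green if free or red if occupied via new dynamic materials, and sets IsReadyToPlace.
; PlaceObject moves a ready unit and registers its tiles as occupied, while ResetLocation restores its BeginPlay position.
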(event `self.ReceiveBeginPlay`
  (set `self.initialLocation` (`SceneComponent.K2_GetComponentLocation` (`self.DefaultSceneRoot`))))

(fn `ChangeGridStatus`
  (params (isValid :type Boolean) (meshIndex :type Integer))
  (bind _output (`|GetArrayItem` (`self.MeshArr`) meshIndex))
  (`/Engine/EditorBlueprintResources/StandardMacros.IsValid` _output
    (:`Is Valid`
      (if isValid
        (bind _returnvalue (`KismetMaterialLibrary.CreateDynamicMaterialInstance` "/Game/Materials/M_GridUnit.M_GridUnit"))
        (`MaterialInstanceDynamic.SetVectorParameterValue` _returnvalue "GridColor" (struct :`G` 1.0 :`A` 1.0))
        (`MaterialInstanceDynamic.SetScalarParameterValue` _returnvalue "Emission" 100.0)
        (`PrimitiveComponent.SetMaterial` _output 0 _returnvalue)
        (else
          (bind _returnvalue_2 (`KismetMaterialLibrary.CreateDynamicMaterialInstance` "/Game/Materials/M_GridUnit.M_GridUnit"))
          (`MaterialInstanceDynamic.SetVectorParameterValue` _returnvalue_2 "GridColor" (struct :`R` 1.0 :`A` 1.0))
          (`MaterialInstanceDynamic.SetScalarParameterValue` _returnvalue_2 "Emission" 100.0)
          (`PrimitiveComponent.SetMaterial` _output 0 _returnvalue_2))))))

(fn `CheckReadyToPlace`
  (params (Grid :type "/Game/Blueprints/BP_GridActor Object Reference") (RequiredLocation :type "Vector Structure"))
  (returns (isOccupied :type Boolean))
  (bind _isoccupied (`/Game/Blueprints/BP_GridActor.CheckOccupiedGrid` Grid RequiredLocation))
  (return _isoccupied))

(fn `GetGridMeshes`
  (returns (MeshArr :type "Array of StaticMeshComponent Object Reference"))
  (return (`self.MeshArr`)))

(fn `OnCheckingGridStatus`
  (params (grid :type "/Game/Blueprints/BP_GridActor Object Reference"))
  (locals (isGridReady :type Boolean :default true))
  (for (_array_element _array_index) (`self.MeshArr`)
    (bind _returnvalue (not (`self.CheckReadyToPlace` grid (`SceneComponent.K2_GetComponentLocation` _array_element))))
    (`self.ChangeGridStatus` _returnvalue _array_index)
    (set `local.isGridReady` (and _returnvalue (`local.isGridReady`))))
  (set `self.isReadyToPlace` (`local.isGridReady`)))

(fn `PlaceObject`
  (params (newLocation :type "Vector Structure") (GridMap :type "/Game/Blueprints/BP_GridActor Object Reference"))
  (returns (isReadyToPlace :type Boolean))
  (bind _isreadytoplace (`self.isReadyToPlace`))
  (if _isreadytoplace
    (`SceneComponent.K2_SetWorldLocation` (`self.DefaultSceneRoot`) newLocation false true)
    (for _array_element (`self.MeshArr`)
      (`/Game/Blueprints/BP_GridActor.AddOccupiedGrid` GridMap (`SceneComponent.K2_GetComponentLocation` _array_element))))
  (return _isreadytoplace))

(fn `ResetLocation`
  (`SceneComponent.K2_SetWorldLocation` (`self.DefaultSceneRoot`) (`self.initialLocation`) false true))

(fn `UserConstructionScript`
  (bind (_returnvalue_x _returnvalue_y _returnvalue_z) (`KismetMathLibrary.BreakVector` (`SceneComponent.K2_GetComponentLocation` (`self.GridMeshParent`))))
  (`KismetArrayLibrary.Array_Clear` (`self.MeshArr`))
  (for _index (range (`self.Grid_X`))
    (for _index_2 (range (`self.Grid_Y`))
      (bind _returnvalue (`AddComponent|NODE_AddStaticMeshComponent-0`))
      (bind _returnvalue_2 (`PrimitiveComponent.CreateDynamicMaterialInstance` _returnvalue 0 "/Game/Materials/M_GridUnit.M_GridUnit" "None"))
      (`MaterialInstanceDynamic.SetVectorParameterValue` _returnvalue_2 "GridColor" (struct :`R` 1.0 :`A` 1.0))
      (`MaterialInstanceDynamic.SetScalarParameterValue` _returnvalue_2 "Emission" 100.0)
      (`SceneComponent.K2_SetWorldTransform` _returnvalue (`KismetMathLibrary.MakeTransform` (`KismetMathLibrary.MakeVector` (+ (`KismetMathLibrary.Conv_IntToDouble` (* _index_2 (`self.TileSize`))) _returnvalue_x) (+ (`KismetMathLibrary.Conv_IntToDouble` (* _index (`self.TileSize`))) _returnvalue_y) _returnvalue_z)) false false)
      (`KismetArrayLibrary.Array_AddUnique` (`self.MeshArr`) _returnvalue)
      (`SceneComponent.K2_AttachToComponent` _returnvalue (`self.GridMeshParent`) "None" "KeepRelative" "KeepRelative" "KeepRelative" true)))
  (for _ (`self.MeshArr`)
    _))